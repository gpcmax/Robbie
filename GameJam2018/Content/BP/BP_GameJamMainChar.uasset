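; BP_GameJamMainChar is the game jam's player character, handling intro, climbing animation, movement audio and a pulse radius.
; BeginPlay disables input and holds then plays a get-up montage, opening a Tick gate that re-enables input once it ends.
; Tick also plays the climb montage on ladders and toggles audio by speed.
; Pulse rescales PulseRadius, while the health-based death and climb-stop logic are unconnected.
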(event EventBeginPlay
  (Input|DisableInput (Game|GetPlayerController 0))
  (Animation|PlayAnimMontage "/Game/CharacterModel/Anims/GetUp.GetUp" 0.0 "None")
  (Utilities|FlowControl|Delay 2.0)
  (Animation|PlayAnimMontage "/Game/CharacterModel/Anims/GetUp.GetUp" 1.0 "None")
  (Utilities|FlowControl|Gate true) ; enters at Open
)

(event EventTick
  (params (DeltaSeconds :type Float%20%28single-precision%29))
  (bind _audio (Variables|Default|GetAudio))
  (Utilities|FlowControl|Sequence
    (:then_0
      (if (Variables|Default|GetbIsOnLadder)
        (Animation|PlayAnimMontage "/Game/CharacterModel/Anims/RobbyClimb_Anim_Montage.RobbyClimb_Anim_Montage" 1.0 "None")))
    (:then_1
      (Utilities|FlowControl|Gate true
        (:Exit
          (if (not (Animation|Montage|MontageIsPlaying (Components|SkeletalMesh|GetAnimInstance (Variables|Character|GetMesh)) "/Game/CharacterModel/Anims/GetUp.GetUp"))
            (Input|EnableInput (Game|GetPlayerController 0))))))
    (:then_2
      (if (> (Math|Vector|VectorLength (Transformation|GetVelocity)) 2e+01)
        (Utilities|FlowControl|DoOnce false :!label _label
          (:Completed
            (Audio|Components|Audio|Play _audio 0.0)))
        (else
          (Audio|Components|Audio|Stop _audio)
          (goto _label Reset))))))

(fn ConstructionScript)

(fn Pulse
  (params (NewScale :type Vector))
  (Transformation|SetWorldTransform (Variables|Default|GetPulseRadius) (Math|Transform|MakeTransform "0, 0, 0" "0, 0, 0" NewScale) false false))