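; BP_Ladder is a ladder actor that automatically carries BP_GameJamMainChar along a climb path when the character overlaps its box.
; On overlap, a DoOnce-guarded timeline flags the character as on a ladder and drives its world location from a scene anchor plus a curve, with Z scaled by a height variable.
; The gate resets when the timeline finishes, and ending overlap clears the flag and restores walking movement.
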(event OnComponentBeginOverlap(Box)
  (params (OverlappedComponent :type Primitive%20Component%20Object%20Reference) (OtherActor :type Actor%20Object%20Reference) (OtherComp :type Primitive%20Component%20Object%20Reference) (OtherBodyIndex :type Integer) (bFromSweep :type Boolean) (SweepResult :type Hit%20Result%20Structure%20%28by%20ref%29))
  (Utilities|FlowControl|DoOnce false :!label _label
    (:Completed
      (bind _asbp_game_jam_main_char (Utilities|Casting|CastToBP_GameJamMainChar OtherActor))
      (Variables|/Script/GameJam2018.GameJamMainChar|SetbIsOnLadder _asbp_game_jam_main_char true)
      (bind _location (Timeline|LadderTimeline PlayFromStart)
        (:Update
          (Transformation|SetWorldLocationAndRotation (Variables|/Script/Engine.Actor|GetRootComponent _asbp_game_jam_main_char) (+ (Transformation|GetWorldLocation (Variables|Default|GetScene)) (Math|Vector|MakeVector (.x _location) (.y _location) (* (.z _location) (Variables|Default|GetLadderHeighVar)))) (Transformation|GetWorldRotation (Variables|/Script/Engine.Actor|GetRootComponent _asbp_game_jam_main_char)) false false))
        (:Finished
          (goto _label Reset))))))

(event OnComponentEndOverlap(Box)
  (params (OverlappedComponent :type Primitive%20Component%20Object%20Reference) (OtherActor :type Actor%20Object%20Reference) (OtherComp :type Primitive%20Component%20Object%20Reference) (OtherBodyIndex :type Integer))
  (bind _asbp_game_jam_main_char (Utilities|Casting|CastToBP_GameJamMainChar OtherActor))
  (Variables|/Script/GameJam2018.GameJamMainChar|SetbIsOnLadder _asbp_game_jam_main_char false)
  (Pawn|Components|CharacterMovement|SetMovementMode (Variables|/Script/Engine.Character|GetCharacterMovement _asbp_game_jam_main_char) "MOVE_Walking" 0)
  (Utilities|FlowControl|Delay 2.0))

(fn ConstructionScript)