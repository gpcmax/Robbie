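; Friendly buddy AI character that follows the player when SetFollow turns following on and deactivates otherwise.
; Tick polls the flag through two DoOnce nodes that re-arm each other, playing deactivate or reactivate montages once per switch and halting movement on deactivation.
; While following, a Gate opened once the reactivate montage finishes drives AIMoveTo toward the player.
; A separate Pulse function rescales the PulseRadius component.
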(event Custom|SetFollow
  (params (NewParam :type Boolean))
  (Variables|Default|SetFollowsPlayer NewParam))

(event EventBeginPlay
  (Animation|PlayAnimMontage "/Game/CharacterModel/Anims/BuddyDectivate__Anim_Montage.BuddyDectivate__Anim_Montage" 1.0 "None")
  (Components|Movement|StopMovementImmediately (Variables|Character|GetCharacterMovement))
  (Utilities|FlowControl|DoOnce false) ; enters at Reset
)

(event EventTick
  (params (DeltaSeconds :type Float%20%28single-precision%29))
  (if (Variables|Default|GetFollowsPlayer)
    (Utilities|FlowControl|Sequence
      (:then_0
        (Utilities|FlowControl|DoOnce false :!label _label
          (:Completed
            (Animation|Montage|MontageStop (Components|SkeletalMesh|GetAnimInstance (Variables|Character|GetMesh)) 0.2 "/Game/CharacterModel/Anims/BuddyDectivate__Anim_Montage.BuddyDectivate__Anim_Montage")
            (Animation|PlayAnimMontage "/Game/CharacterModel/Anims/BuddyReactivate_Anim_Montage.BuddyReactivate_Anim_Montage" 1.0 "None")
            (goto _label_3 Reset))))
      (:then_1
        (if (not (Animation|Montage|MontageIsPlaying (Components|SkeletalMesh|GetAnimInstance (Variables|Character|GetMesh)) "/Game/CharacterModel/Anims/BuddyReactivate_Anim_Montage.BuddyReactivate_Anim_Montage"))
          (goto _label_2 Open)))
      (:then_2
        (Utilities|FlowControl|Gate true :!label _label_2
          (:Exit
            (bind _asbp_game_jam_main_char (Utilities|Casting|CastToBP_GameJamMainChar (Game|Player|GetPlayerPawn 0)))
            (AI|AIMoveTo self "0, 0, 0" _asbp_game_jam_main_char 1e+02 false)))))
    (else
      (Utilities|FlowControl|DoOnce false :!label _label_3
        (:Completed
          (Animation|PlayAnimMontage "/Game/CharacterModel/Anims/BuddyDectivate__Anim_Montage.BuddyDectivate__Anim_Montage" 1.0 "None")
          (Components|Movement|StopMovementImmediately (Variables|Character|GetCharacterMovement))
          (goto _label Reset))))))

(fn ConstructionScript)

(fn Pulse
  (params (NewScale :type Vector))
  (Transformation|SetWorldTransform (Variables|Default|GetPulseRadius) (Math|Transform|MakeTransform "0, 0, 0" "0, 0, 0" NewScale) false false))